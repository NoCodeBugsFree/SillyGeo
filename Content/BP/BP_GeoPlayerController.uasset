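; BP_GeoPlayerController is a player controller that manages the game's HUD and its win and lose endings.
; On BeginPlay it creates WBP_HUD and adds it to the viewport, then forwards UpdateHUD calls to the widget.
; The win and lose events trigger the matching HUD display and remove the widget after a delay.
; Winning also quits the game after a further delay, while losing does not.
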(event EventBeginPlay
  ;[0 0.08263 1] HUD
  (bind _returnvalue (UserInterface|CreateWidget "/Game/HUD/WBP_HUD.WBP_HUD_C"))
  (bind _output_get (Variables|Default|SetHUD _returnvalue))
  (UserInterface|Viewport|AddtoViewport _output_get 0))

(event EventLosetheGame
  ;[0 0.08263 1] Win/Lose
  (Default|LosetheGame (Variables|Default|GetHUD))
  (Utilities|FlowControl|Delay 3.0)
  (Widget|RemovefromParent (Variables|Default|GetHUD)))

(event EventWintheGame
  ;[0 0.08263 1] Win/Lose
  (Default|WintheGame (Variables|Default|GetHUD))
  (Utilities|FlowControl|Delay 3.0)
  (Widget|RemovefromParent (Variables|Default|GetHUD))
  (Utilities|FlowControl|Delay 3.0)
  (Game|QuitGame 0 "Quit"))

(event EventUpdateHUD
  (bind _hud (Variables|Default|GetHUD))
  ;[0 0.08263 1] HUD
  (Utilities|IsValid _hud
    (:Is%20Valid
      (Default|UpdateHUD _hud))))

(fn ConstructionScript)