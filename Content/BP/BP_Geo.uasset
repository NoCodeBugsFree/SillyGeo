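; BP_Geo handles the visual effect for switching weapons, shown as interchangeable wing meshes.
; A WeaponSwitch timeline drives both the wings' material opacity and their scale from one Scale track.
; Its Swap event track sets the mesh for CurrentWeapon from the wing list built in the construction script.
; When the timeline finishes, a short delay re-enables weapon switching.
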(event EventWeaponSwitchFX
  ;[1 0.1807 0] Weapon Switch FX
  (bind _scale (Timeline|WeaponSwitch PlayFromStart)
    (:Update
      (Rendering|Material|SetScalarParameterValue (Variables|Default|GetWingsDynamicMaterial) "Opacity" _scale :!class /Script/Engine.MaterialInstanceDynamic)
      (Transformation|SetRelativeScale3D (Variables|Default|GetWeaponWings) (Math|Conversions|ToVector(Float) _scale)))
    (:Finished
      (Utilities|FlowControl|Delay 0.2)
      (Variables|Default|SetbCanSwitchWeapon true))
    (:Swap
      (Components|StaticMesh|SetStaticMesh (Variables|Default|GetWeaponWings) (Utilities|Array|Get(acopy) (Variables|Default|GetWingList) (Variables|Default|GetCurrentWeapon))))))

(fn ConstructionScript
  (Variables|Default|SetWingList (Utilities|Array|MakeArray "/Game/Player/Meshes/SM_Wing_Simple.SM_Wing_Simple" "/Game/Player/Meshes/SM_Wing_Butterfly.SM_Wing_Butterfly" "/Game/Player/Meshes/SM_Wing_Jet.SM_Wing_Jet" "/Game/Player/Meshes/SM_Wing_Discus.SM_Wing_Discus")))